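; BP_enemy is an enemy actor that hurts the player on contact and can be shot for points.
; Overlapping BP_Player removes one health point, updates the health bar, flags death and shows restart at zero, adds a Hurt widget, then destroys the enemy.
; A BP_BOOLET hit increments the player's score and its display, raises their forward speed modifier, and destroys the enemy, so each kill speeds up the player.
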(event `self.StaticMeshComponent.OnComponentBeginOverlap`
  (params (OverlappedComponent :type "PrimitiveComponent Object Reference") (OtherActor :type "Actor Object Reference") (OtherComp :type "PrimitiveComponent Object Reference") (OtherBodyIndex :type Integer) (bFromSweep :type Boolean) (SweepResult :type "HitResult Structure (by ref)"))
  (bind _asbp_player (cast `/Game/InfiniteMatrix/Blueprints/BP_Player` OtherActor))
  (bind _returnvalue (+ -1 (`/Game/InfiniteMatrix/Blueprints/BP_Player.health_points` _asbp_player)))
  (if (not (> _returnvalue 5))
    (bind _output_get (set `/Game/InfiniteMatrix/Blueprints/BP_Player.health_points` _returnvalue _asbp_player))
    (`ProgressBar.SetPercent` (`/Game/InfiniteMatrix/UI/health.ProgressBar_132` (`/Game/InfiniteMatrix/Blueprints/BP_Player.Health` _asbp_player)) (`KismetMathLibrary.SafeDivide` (`KismetMathLibrary.Conv_IntToDouble` _output_get) 5.0))
    (if (== _output_get 0)
      (set `/Game/InfiniteMatrix/Blueprints/BP_Player.IsDead` true _asbp_player)
      (`/Game/InfiniteMatrix/Blueprints/BP_Player.DisplayRestart` _asbp_player)))
  (bind _returnvalue_2 (`|CreateWidget` "/Game/InfiniteMatrix/UI/hurt.hurt_C"))
  (`UserWidget.AddToViewport` _returnvalue_2 1)
  (`self.K2_DestroyActor` :!label _label))

(event `self.StaticMeshComponent.OnComponentHit`
  (params (HitComponent :type "PrimitiveComponent Object Reference") (OtherActor :type "Actor Object Reference") (OtherComp :type "PrimitiveComponent Object Reference") (NormalImpulse :type "Vector Structure") (Hit :type "HitResult Structure (by ref)"))
  (bind _asbp_boolet (cast `/Game/InfiniteMatrix/Blueprints/BP_BOOLET` OtherActor))
  (`|ExecutionSequence`
    (:`then_0`
      (bind _asbp_player (cast `/Game/InfiniteMatrix/Blueprints/BP_Player` (`GameplayStatics.GetPlayerPawn` 0)))
      (bind _result (`/Engine/EditorBlueprintResources/StandardMacros.IncrementInt` (`/Game/InfiniteMatrix/Blueprints/BP_Player.score` _asbp_player))
        (:`  `
          (`EditableText.SetText` (`/Game/InfiniteMatrix/UI/score.EditableText` (`/Game/InfiniteMatrix/Blueprints/BP_Player.score_display` _asbp_player)) (`KismetTextLibrary.Conv_StringToText` (`KismetStringLibrary.Concat_StrStr` (`/Game/InfiniteMatrix/Blueprints/BP_Player.score_string` _asbp_player) (`KismetStringLibrary.Conv_IntToString` _result))))
          (set `/Game/InfiniteMatrix/Blueprints/BP_Player.forward_speed_mod` (+ (`/Game/InfiniteMatrix/Blueprints/BP_Player.forward_speed_mod` _asbp_player) 25.0) _asbp_player))))
    (:`then_1`
      (goto _label))))

(fn `UserConstructionScript`)