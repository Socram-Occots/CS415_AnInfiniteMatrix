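; BP_health_pack is a health pickup actor that restores one health point to the player on contact.
; Its static mesh's begin-overlap event casts to BP_Player, adds the point unless that would exceed the maximum of five, and updates the player's health progress bar directly.
; The pack destroys itself on any player overlap, even when health is already full.
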(event `self.StaticMeshComponent.OnComponentBeginOverlap`
  (params (OverlappedComponent :type "PrimitiveComponent Object Reference") (OtherActor :type "Actor Object Reference") (OtherComp :type "PrimitiveComponent Object Reference") (OtherBodyIndex :type Integer) (bFromSweep :type Boolean) (SweepResult :type "HitResult Structure (by ref)"))
  (bind _asbp_player (cast `/Game/InfiniteMatrix/Blueprints/BP_Player` OtherActor))
  (bind _returnvalue (+ 1 (`/Game/InfiniteMatrix/Blueprints/BP_Player.health_points` _asbp_player)))
  (if (not (> _returnvalue 5))
    (bind _output_get (set `/Game/InfiniteMatrix/Blueprints/BP_Player.health_points` _returnvalue _asbp_player))
    (`ProgressBar.SetPercent` (`/Game/InfiniteMatrix/UI/health.ProgressBar_132` (`/Game/InfiniteMatrix/Blueprints/BP_Player.Health` _asbp_player)) (`KismetMathLibrary.SafeDivide` (`KismetMathLibrary.Conv_IntToDouble` _output_get) 5.0)))
  (`self.K2_DestroyActor`))

(event `self.ReceiveTick`
  (params (DeltaSeconds :type "Float (single-precision)")))

(fn `UserConstructionScript`)